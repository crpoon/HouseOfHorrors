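; BP_JumpScareTriggerDoor is a House of Horror trigger that plays a jump scare when the player character overlaps it.
; It spawns a BP_Scream 100 units in front of the VR camera, yawed 180 degrees from the camera's rotation, and starts the scream.
; A flag blocks retriggering until a three-second delay ends and the scream is destroyed.
; The trigger then optionally destroys itself for one-time use.
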(event `self.ReceiveActorBeginOverlap`
  (params (OtherActor :type "Actor Object Reference"))
  (if (not (`self.isPlayingJumpScream`))
    (bind _asbp_ho_hchar (cast `/Game/HouseOfHorror/Blueprints/Character/BP_HoHChar` OtherActor))
    (bind (_location _forward_vector) (`/Game/HouseOfHorror/Blueprints/Character/LayoutVRUtilityFunctions.Get Player VR Camera Properties`))
    (bind _returnvalue (`|SpawnActorFromClass` "/Game/HouseOfHorror/Blueprints/Characters/BP_Scream.BP_Scream_C" (`KismetMathLibrary.MakeTransform` (+ _location (* _forward_vector 100)) (`KismetMathLibrary.MakeRotator` (.roll (`SceneComponent.K2_GetComponentRotation` (`/Game/HouseOfHorror/Blueprints/Character/BP_HoHChar.Camera` _asbp_ho_hchar))) (.pitch (`SceneComponent.K2_GetComponentRotation` (`/Game/HouseOfHorror/Blueprints/Character/BP_HoHChar.Camera` _asbp_ho_hchar))) (+ (.yaw (`SceneComponent.K2_GetComponentRotation` (`/Game/HouseOfHorror/Blueprints/Character/BP_HoHChar.Camera` _asbp_ho_hchar))) 180.0))) "AlwaysSpawn" "OverrideRootScale"))
    (`/Game/HouseOfHorror/Blueprints/Characters/BP_Scream.SetScream` _returnvalue true)
    (`/Game/HouseOfHorror/Blueprints/Characters/BP_Scream.Scream` _returnvalue)
    (set `self.isPlayingJumpScream` true)
    (`KismetSystemLibrary.Delay` 3.0)
    (`self.K2_DestroyActor` _returnvalue)
    (set `self.isPlayingJumpScream` false)
    (if (`self.DestroyOnceUsed`)
      (`self.K2_DestroyActor`))))

(fn `UserConstructionScript`)