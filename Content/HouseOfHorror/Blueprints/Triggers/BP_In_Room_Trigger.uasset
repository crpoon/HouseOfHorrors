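; Room trigger volume that tells the player and AI characters which room they are currently in.
; On box overlap it writes itself into the CurrentRoom of the entering BP_HoHChar or BP_AICharacter.
; On exit it clears CurrentRoom for BP_HoHChar only, without checking whether another room has already set it, so AI characters keep their last room.
; Disconnected debug prints reference each room's name and neighbour list.
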(event `self.ReceiveBeginPlay`)

(event `self.ReceiveActorBeginOverlap`
  (params (OtherActor :type "Actor Object Reference")))

(event `self.ReceiveTick`
  (params (DeltaSeconds :type "Float (single-precision)")))

(event `self.Box.OnComponentBeginOverlap`
  (params (OtherActor :type "Actor Object Reference") (OtherComp :type "PrimitiveComponent Object Reference") (OtherBodyIndex :type Integer) (bFromSweep :type Boolean) (SweepResult :type "HitResult Structure (by ref)"))
  (bind _asbp_ho_hchar (cast `/Game/HouseOfHorror/Blueprints/Character/BP_HoHChar` OtherActor)
    (:`then`
      (bind _output_get (set `/Game/HouseOfHorror/Blueprints/Character/BP_HoHChar.CurrentRoom` self _asbp_ho_hchar)))
    (:`CastFailed`
      (bind _asbp_aicharacter (cast `/Game/HouseOfHorror/Blueprints/Characters/BP_AICharacter` OtherActor))
      (bind _output_get_2 (set `/Game/HouseOfHorror/Blueprints/Characters/BP_AICharacter.CurrentRoom` self _asbp_aicharacter)))))

(event `self.Box.OnComponentEndOverlap`
  (params (OtherActor :type "Actor Object Reference") (OtherComp :type "PrimitiveComponent Object Reference") (OtherBodyIndex :type Integer))
  (bind _asbp_ho_hchar (cast `/Game/HouseOfHorror/Blueprints/Character/BP_HoHChar` OtherActor))
  (set `/Game/HouseOfHorror/Blueprints/Character/BP_HoHChar.CurrentRoom` null _asbp_ho_hchar))

(fn `UserConstructionScript`)