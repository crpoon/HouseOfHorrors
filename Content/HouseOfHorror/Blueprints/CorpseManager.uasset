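; Manager actor that periodically spawns corpse enemies near the player in the House of Horror game.
; A looping timer picks the player's room, or a random neighbour if it is an intersection, then randomly spawns in an adjacent room while under the active corpse cap.
; Types are drawn randomly from an available pool and spawned as behavior-tree AI holding a manager reference and ID.
; Functions let the count be decremented and IDs returned to the pool.
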(event `self.ReceiveBeginPlay`
  (`KismetSystemLibrary.K2_SetTimer` null "SpawnCorpse" 5.0 true))

(event `self.ReceiveActorBeginOverlap`
  (params (OtherActor :type "Actor Object Reference")))

(event `self.ReceiveTick`
  (params (DeltaSeconds :type "Float (single-precision)")))

(fn `CanSpawn`
  (params (currentRoom :type "/Game/HouseOfHorror/Blueprints/In_Room_Trigger Object Reference"))
  (returns (canSpawn :type Boolean))
  (return (and (!= currentRoom null) (< (`self.NumActiveCorpses`) 2) (> (`KismetMathLibrary.RandomFloatInRange` 0.0 1.0) 0.5))))

(fn `DecrementNumActiveCorpes`
  (`/Engine/EditorBlueprintResources/StandardMacros.DecrementInt` (`self.NumActiveCorpses`)
    (:`  `
      (return))))

(fn `GetCorpseTypeToSpawn`
  (returns (type :type Integer))
  (bind _availablecorpsestocall (`self.AvailableCorpsesToCall`))
  (bind _output_get (set `self.IndexToRemove` (`KismetMathLibrary.RandomIntegerInRange` 0 (- (`KismetArrayLibrary.Array_Length` _availablecorpsestocall) 1))))
  (bind _output_get_2 (set `self.Spawning` (`KismetArrayLibrary.Array_Get` _availablecorpsestocall _output_get)))
  (`KismetArrayLibrary.Array_Remove` _availablecorpsestocall _output_get)
  (return _output_get_2))

(fn `GetSpawnLocation`
  (params (currentRoom :type "/Game/HouseOfHorror/Blueprints/In_Room_Trigger Object Reference"))
  (returns (location :type "Vector Structure"))
  (bind _neighbours (`/Game/HouseOfHorror/Blueprints/In_Room_Trigger.Neighbours` currentRoom))
  (return (+ (`self.K2_GetActorLocation` (`KismetArrayLibrary.Array_Get` _neighbours (`KismetMathLibrary.RandomIntegerInRange` 0 (- (`KismetArrayLibrary.Array_Length` _neighbours) 1)))) (0.0 0.0 70.0))))

(fn `SetCorpseAvailable`
  (params (id :type Integer))
  (`KismetArrayLibrary.Array_Add` (`self.AvailableCorpsesToCall`) id))

(fn `SpawnCorpse`
  (bind _asbp_ho_hchar (cast `/Game/HouseOfHorror/Blueprints/Character/BP_HoHChar` (`GameplayStatics.GetPlayerPawn` 0)))
  (bind _currentroom (`/Game/HouseOfHorror/Blueprints/Character/BP_HoHChar.CurrentRoom` _asbp_ho_hchar))
  (if (`/Game/HouseOfHorror/Blueprints/In_Room_Trigger.IsIntersection` _currentroom)
    (bind _neighbours (`/Game/HouseOfHorror/Blueprints/In_Room_Trigger.Neighbours` _currentroom))
    (bind _output_get (set `self.centralRoom` (`KismetArrayLibrary.Array_Get` _neighbours (`KismetMathLibrary.RandomIntegerInRange` 0 (- (`KismetArrayLibrary.Array_Length` _neighbours) 1)))))
    (else
      (set `self.centralRoom` _currentroom)))
  (bind _canspawn (`self.CanSpawn` _output_get))
  (if _canspawn
    (bind _location (`self.GetSpawnLocation` (`self.centralRoom`)))
    (`/Engine/EditorBlueprintResources/StandardMacros.IncrementInt` (`self.NumActiveCorpses`)
      (:`  `
        (bind _type (`self.GetCorpseTypeToSpawn`))
        (`self.SpawnCorpseOfType` _type _location)))))

(fn `SpawnCorpseOfType`
  (params (type :type Integer) (location :type "Vector Structure"))
  (switch `int` type
    (:`0`
      (bind _returnvalue (`AIBlueprintHelperLibrary.SpawnAIFromClass` "/Game/HouseOfHorror/Blueprints/Characters/BP_Corpse_Bob.BP_Corpse_Bob_C" "/Game/HouseOfHorror/Blueprints/AI/BehaviourTree/BT_Follower.BT_Follower" location))
      (bind _asbp_corpse_bob (cast `/Game/HouseOfHorror/Blueprints/Characters/BP_Corpse_Bob` _returnvalue))
      (set `/Game/HouseOfHorror/Blueprints/Characters/BP_AICharacter.CorpseManager` self _asbp_corpse_bob)
      (bind _output_get (set `/Game/HouseOfHorror/Blueprints/Characters/BP_AICharacter.CorpseId` 0 _asbp_corpse_bob))
      (`KismetSystemLibrary.PrintString` (`KismetStringLibrary.Concat_StrStr` "Spawn corpse " (`KismetStringLibrary.Conv_IntToString` _output_get))))
    (:`1`
      (bind _returnvalue_2 (`AIBlueprintHelperLibrary.SpawnAIFromClass` "/Game/HouseOfHorror/Blueprints/Characters/BP_Corpse_Creep.BP_Corpse_Creep_C" "/Game/HouseOfHorror/Blueprints/AI/BehaviourTree/BT_Follower.BT_Follower" location))
      (bind _asbp_corpse_creep (cast `/Game/HouseOfHorror/Blueprints/Characters/BP_Corpse_Creep` _returnvalue_2))
      (set `/Game/HouseOfHorror/Blueprints/Characters/BP_AICharacter.CorpseManager` self _asbp_corpse_creep)
      (bind _output_get_2 (set `/Game/HouseOfHorror/Blueprints/Characters/BP_AICharacter.CorpseId` 1 _asbp_corpse_creep))
      (`KismetSystemLibrary.PrintString` (`KismetStringLibrary.Concat_StrStr` "Spawn corpse " (`KismetStringLibrary.Conv_IntToString` _output_get_2))))
    (:`2`
      (bind _returnvalue_3 (`AIBlueprintHelperLibrary.SpawnAIFromClass` "/Game/HouseOfHorror/Blueprints/Characters/BP_Corpse_FormerGuard.BP_Corpse_FormerGuard_C" "/Game/HouseOfHorror/Blueprints/AI/BehaviourTree/BT_Follower.BT_Follower" location))
      (bind _asbp_corpse_former_guard (cast `/Game/HouseOfHorror/Blueprints/Characters/BP_Corpse_FormerGuard` _returnvalue_3))
      (set `/Game/HouseOfHorror/Blueprints/Characters/BP_AICharacter.CorpseManager` self _asbp_corpse_former_guard)
      (bind _output_get_3 (set `/Game/HouseOfHorror/Blueprints/Characters/BP_AICharacter.CorpseId` 2 _asbp_corpse_former_guard))
      (`KismetSystemLibrary.PrintString` (`KismetStringLibrary.Concat_StrStr` "Spawn corpse " (`KismetStringLibrary.Conv_IntToString` _output_get_3))))
    (:`3`
      (bind _returnvalue_4 (`AIBlueprintHelperLibrary.SpawnAIFromClass` "/Game/HouseOfHorror/Blueprints/Characters/BP_Scream.BP_Scream_C" "/Game/HouseOfHorror/Blueprints/AI/BehaviourTree/BT_Follower_Screamer.BT_Follower_Screamer" location))
      (bind _asbp_scream (cast `/Game/HouseOfHorror/Blueprints/Characters/BP_Scream` _returnvalue_4))
      (set `/Game/HouseOfHorror/Blueprints/Characters/BP_AICharacter.CorpseManager` self _asbp_scream)
      (bind _output_get_4 (set `/Game/HouseOfHorror/Blueprints/Characters/BP_AICharacter.CorpseId` 3 _asbp_scream))
      (`KismetSystemLibrary.PrintString` (`KismetStringLibrary.Concat_StrStr` "Spawn corpse " (`KismetStringLibrary.Conv_IntToString` _output_get_4))))))

(fn `UserConstructionScript`)