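; Behavior tree task that picks a random reachable point near the AI's controlled pawn in House of Horror.
; On execute it casts the owner to BP_AIController on first use and caches the reference.
; It then finds a navigable point within a fixed radius of the pawn, writes it to the TargetLocation blackboard key and finishes successfully.
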(event `self.ReceiveExecute`
  (params (OwnerActor :type "Actor Object Reference"))
  (if (not (!= (`self.AIControllerRef`) null))
    (bind _asbp_aicontroller (cast `/Game/HouseOfHorror/Blueprints/AI/BP_AIController` OwnerActor))
    (set `self.AIControllerRef` _asbp_aicontroller))
  (`BTFunctionLibrary.SetBlackboardValueAsVector` (`self.TargetLocation`) (`NavigationSystem.GetRandomReachablePointInRadius` (`Actor.K2_GetActorLocation` (`Controller.K2_GetPawn` (`self.AIControllerRef`))) 1000.0))
  (`self.FinishExecute` true))