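; Behavior tree tick logic for BP_AIController that maintains the SafeDistance blackboard value between the controlled pawn and its TargetToFollow actor.
; When SafeDistance is zero, it seeds the value with the current pawn-to-target distance, clamped to a 300-unit minimum.
; Afterwards it only shrinks the value as the pawn gets closer, ignoring distances at or below that minimum.
; Each tick also prints the stored value for debugging.
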(event `self.ReceiveTick`
  (params (OwnerActor :type "Actor Object Reference") (DeltaSeconds :type "Float (single-precision)"))
  (bind _safedistance (`self.SafeDistance`))
  (bind _returnvalue (`BTFunctionLibrary.GetBlackboardValueAsFloat` (`self.SafeDistance`)))
  (bind _returnvalue_2 (`KismetMathLibrary.VSize` (- (`Actor.K2_GetActorLocation` (`BTFunctionLibrary.GetBlackboardValueAsActor` (`self.TargetToFollow`))) (`Actor.K2_GetActorLocation` (`Controller.K2_GetPawn` (`self.AIControllerRef`))))))
  (bind _asbp_aicontroller (cast `/Game/HouseOfHorror/Blueprints/AI/BP_AIController` OwnerActor))
  (set `self.AIControllerRef` _asbp_aicontroller)
  (`KismetSystemLibrary.PrintString` (`KismetStringLibrary.Conv_DoubleToString` _returnvalue))
  (if (`KismetMathLibrary.NearlyEqual_FloatFloat` _returnvalue)
    (if (> _returnvalue_2 300.0)
      (`BTFunctionLibrary.SetBlackboardValueAsFloat` _safedistance _returnvalue_2)
      (else
        (`BTFunctionLibrary.SetBlackboardValueAsFloat` _safedistance 300.0)))
    (elif (and (< _returnvalue_2 (`BTFunctionLibrary.GetBlackboardValueAsFloat` (`self.SafeDistance`))) (> _returnvalue_2 300.0))
      (`BTFunctionLibrary.SetBlackboardValueAsFloat` _safedistance _returnvalue_2))))