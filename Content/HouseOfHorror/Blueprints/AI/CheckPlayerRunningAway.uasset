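; Behavior tree node that makes a screamer AI raise an alarm when its followed target runs away.
; On tick, it seeds an unset SafeDistance blackboard value from the current pawn-to-TargetToFollow distance plus a margin.
; Once the target exceeds that distance, it flags IsScreamerCalling on BP_GameInstance, stores the pawn's location as ScreamerPosition and prints a debug message.
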(event `self.ReceiveTick`
  (params (OwnerActor :type "Actor Object Reference") (DeltaSeconds :type "Float (single-precision)"))
  (bind _returnvalue (`Actor.K2_GetActorLocation` (`Controller.K2_GetPawn` (`self.AIControllerRef`))))
  (bind _returnvalue_2 (`KismetMathLibrary.VSize` (- (`Actor.K2_GetActorLocation` (`BTFunctionLibrary.GetBlackboardValueAsActor` (`self.TargetToFollow`))) _returnvalue)))
  (bind _asbp_aicontroller (cast `/Game/HouseOfHorror/Blueprints/AI/BP_AIController` OwnerActor))
  (set `self.AIControllerRef` _asbp_aicontroller)
  (if (< (`BTFunctionLibrary.GetBlackboardValueAsFloat` (`self.SafeDistance`)) 0.1)
    (`BTFunctionLibrary.SetBlackboardValueAsFloat` (`self.SafeDistance`) (+ _returnvalue_2 100.0)))
  (if (> _returnvalue_2 (`BTFunctionLibrary.GetBlackboardValueAsFloat` (`self.SafeDistance`)))
    (bind _asbp_game_instance (cast `/Game/HouseOfHorror/Blueprints/BP_GameInstance` (`GameplayStatics.GetGameInstance`)))
    (set `/Game/HouseOfHorror/Blueprints/BP_GameInstance.IsScreamerCalling` true _asbp_game_instance)
    (set `/Game/HouseOfHorror/Blueprints/BP_GameInstance.ScreamerPosition` _returnvalue _asbp_game_instance)
    (`KismetSystemLibrary.PrintString` "Scream!!!!!!")))