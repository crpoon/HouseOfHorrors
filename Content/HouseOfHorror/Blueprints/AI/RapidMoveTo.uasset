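; RapidMoveTo is a Behavior Tree task that moves the AI's controlled pawn toward the actor stored in the TargetToFollow blackboard key.
; On execute it casts the owner to BP_AIController, caches that reference for later runs, and calls AIMoveTo with a fixed acceptance radius.
; The task finishes only when the move succeeds, as neither a failed move nor a failed cast calls FinishExecute.
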(event `self.ReceiveExecute`
  (params (OwnerActor :type "Actor Object Reference"))
  (if (not (!= (`self.AIControllerRef`) null))
    (bind _asbp_aicontroller (cast `/Game/HouseOfHorror/Blueprints/AI/BP_AIController` OwnerActor))
    (set `self.AIControllerRef` _asbp_aicontroller))
  (`|AIMoveTo` (`Controller.K2_GetPawn` (`self.AIControllerRef`)) (0.0 0.0 0.0) (`BTFunctionLibrary.GetBlackboardValueAsActor` (`self.TargetToFollow`)) 100.0
    (:`OnSuccess`
      (`self.FinishExecute` true))))