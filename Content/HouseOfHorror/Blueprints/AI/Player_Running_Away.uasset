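; Behavior tree decorator for the House of Horror AI that checks whether the followed target, likely the player, has moved too far away.
; It casts the owner to BP_AIController, then measures the distance from the controlled pawn to the TargetToFollow blackboard actor.
; The condition passes when that distance exceeds AcceptableDistance.
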(fn `PerformConditionCheck`
  (params (OwnerActor :type "Actor Object Reference"))
  (returns (ReturnValue :type Boolean))
  (bind _asbp_aicontroller (cast `/Game/HouseOfHorror/Blueprints/AI/BP_AIController` OwnerActor))
  (set `self.AIControllerRef` _asbp_aicontroller)
  (return (> (`KismetMathLibrary.VSize` (- (`Actor.K2_GetActorLocation` (`BTFunctionLibrary.GetBlackboardValueAsActor` (`self.TargetToFollow`))) (`Actor.K2_GetActorLocation` (`Controller.K2_GetPawn` (`self.AIControllerRef`))))) (`self.AcceptableDistance`))))