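; Player character for House of Horror, handling movement and look input, run and crawl, a flashlight toggle, interaction and pausing.
; Run and crawl scale max walk speed by reciprocal multipliers on press and release, mirroring speed, movement state and torch status to BP_GameInstance.
; Interact line-traces from the camera to trigger objective objects or interactable architecture.
; Pause toggles on-screen text; quitting from pause is an unimplemented TODO.
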(event `self.ReceiveBeginPlay`)

(event `self.ReceiveActorBeginOverlap`
  (params (OtherActor :type "Actor Object Reference")))

(event `InputAction|SpeedUp`
  (params (Key :type "Key Structure" :default "AnyKey"))
  (bind _charactermovement (`self.CharacterMovement`))
  (:`Pressed`
    (bind _game_instance (`self.getGameInstance`))
    (set `/Game/HouseOfHorror/Blueprints/BP_GameInstance.isPlayerRunning` true _game_instance)
    (set `self.BaseMoveSpeed` 1.25)
    (bind _output_get (set `CharacterMovementComponent.MaxWalkSpeed` (* (`CharacterMovementComponent.MaxWalkSpeed` _charactermovement) (`self.BaseMoveSpeed`)) _charactermovement :!label _label))
    (bind _game_instance_2 (`self.getGameInstance`))
    (set `/Game/HouseOfHorror/Blueprints/BP_GameInstance.playerSpeed` _output_get _game_instance_2))
  (:`Released`
    (bind _game_instance_3 (`self.getGameInstance`))
    (set `/Game/HouseOfHorror/Blueprints/BP_GameInstance.isPlayerRunning` false _game_instance_3)
    (set `self.BaseMoveSpeed` 0.8)
    (goto _label)))

(event `InputAxis|MoveForward`
  (params (AxisValue :type "Float (single-precision)"))
  ;[1 1 1] Movement + Look
  (`self.AddMovementInput` (`self.GetActorForwardVector`) (* AxisValue (`self.BaseMoveSpeed`))))

(event `InputAxis|MoveRight`
  (params (AxisValue :type "Float (single-precision)"))
  ;[1 1 1] Movement + Look
  (`self.AddMovementInput` (`self.GetActorRightVector`) (* AxisValue (`self.BaseMoveSpeed`))))

(event `InputAction|SlowDown`
  (params (Key :type "Key Structure" :default "AnyKey"))
  (bind _charactermovement (`self.CharacterMovement`))
  (:`Pressed`
    (bind _game_instance (`self.getGameInstance`))
    (set `/Game/HouseOfHorror/Blueprints/BP_GameInstance.isPlayerCrawling` true _game_instance)
    (set `self.BaseMoveSpeed` 0.5)
    (bind _output_get (set `CharacterMovementComponent.MaxWalkSpeed` (* (`CharacterMovementComponent.MaxWalkSpeed` _charactermovement) (`self.BaseMoveSpeed`)) _charactermovement :!label _label_2))
    (bind _game_instance_2 (`self.getGameInstance`))
    (set `/Game/HouseOfHorror/Blueprints/BP_GameInstance.playerSpeed` _output_get _game_instance_2))
  (:`Released`
    (bind _game_instance_3 (`self.getGameInstance`))
    (set `/Game/HouseOfHorror/Blueprints/BP_GameInstance.isPlayerCrawling` false _game_instance_3)
    (set `self.BaseMoveSpeed` 2.0)
    (goto _label_2)))

(event `InputAxis|Turn`
  (params (AxisValue :type "Float (single-precision)"))
  ;[1 1 1] Movement + Look
  (`self.AddControllerYawInput` AxisValue))

(event `InputAxis|LookUp`
  (params (AxisValue :type "Float (single-precision)"))
  ;[1 1 1] Movement + Look
  (`self.AddControllerPitchInput` AxisValue))

(event `InputAxis|TurnRate`
  (params (AxisValue :type "Float (single-precision)"))
  ;[1 1 1] Movement + Look
  (`self.AddControllerYawInput` (* AxisValue (`self.BaseTurnRate`) (`GameplayStatics.GetWorldDeltaSeconds`))))

(event `InputAxis|LookUpRate`
  (params (AxisValue :type "Float (single-precision)"))
  ;[1 1 1] Movement + Look
  (`self.AddControllerPitchInput` (* AxisValue (`self.BaseLookUpRate`) (`GameplayStatics.GetWorldDeltaSeconds`))))

(event `InputAction|LightToggle`
  (params (Key :type "Key Structure" :default "AnyKey"))
  ;[1 1 1] Flashlight
  (:`Pressed`
    (if (`self.LightOn`)
      (`LightComponent.SetIntensity` (`self.SpotLight`) 0.0)
      (set `self.LightOn` false)
      (else
        (`LightComponent.SetIntensity` (`self.SpotLight`) 15000.0)
        (set `self.LightOn` true)))
    (bind _game_instance (`self.getGameInstance`))
    (set `/Game/HouseOfHorror/Blueprints/BP_GameInstance.isTorchlightOn` (`self.LightOn`) _game_instance)))

(event `InputAction|Interact`
  (params (Key :type "Key Structure" :default "AnyKey"))
  (bind _returnvalue (`GameplayStatics.GetPlayerCameraManager` 0))
  (bind _returnvalue_2 (`self.K2_GetActorLocation` _returnvalue))
  ;[1 1 1] Interact
  (:`Pressed`
    (bind (_outhit _returnvalue_3) (`KismetSystemLibrary.LineTraceSingle` :`Start` _returnvalue_2 :`End` (+ _returnvalue_2 (* (`self.GetActorForwardVector` _returnvalue) 250)) :`TraceChannel` "TraceTypeQuery1" :`DrawDebugType` "ForDuration"))
    (if _returnvalue_3
      (bind (_bblockinghit _binitialoverlap _time _location _impactpoint _normal _impactnormal _physmat _hitactor) (`GameplayStatics.BreakHitResult` _outhit))
      (bind _asbp_objective_object (cast `/Game/HouseOfHorror/Blueprints/Objects/BP_ObjectiveObject` _hitactor)
        (:`then`
          (`/Game/HouseOfHorror/Blueprints/Objects/BP_ObjectiveObject.OnCollision` _asbp_objective_object))
        (:`CastFailed`
          (bind _asbp_objective_child (cast `/Game/HouseOfHorror/Blueprints/Objects/BP_ObjectiveChild` _hitactor)
            (:`then`
              (`/Game/HouseOfHorror/Blueprints/Objects/BP_ObjectiveObject.OnCollision` _asbp_objective_child))
            (:`CastFailed`
              (bind _asbp_interactable_architecture (cast `/Game/HouseOfHorror/Blueprints/Architecture/BP_InteractableArchitecture` _hitactor))
              (`/Game/HouseOfHorror/Blueprints/Architecture/BP_Interact.Interact` _asbp_interactable_architecture))))))))

(event `InputAction|Pause` :paused true
  (params (Key :type "Key Structure" :default "AnyKey"))
  (bind _pausetext (`self.PauseText`))
  (bind _pauseoptiontext (`self.PauseOptionText`))
  ;[1 1 1] Pause
  (:`Pressed`
    (if (`GameplayStatics.IsGamePaused`)
      (`GameplayStatics.SetGamePaused` false)
      (`SceneComponent.SetVisibility` _pausetext false false)
      (`SceneComponent.SetVisibility` _pauseoptiontext false false)
      (else
        (`GameplayStatics.SetGamePaused` true)
        (`SceneComponent.SetVisibility` _pausetext true false)
        (`SceneComponent.SetVisibility` _pauseoptiontext true false)))))

(event `InputAction|QuitGameFromPause` :paused true
  (params (Key :type "Key Structure" :default "AnyKey"))
  ;[1 1 1] TODO: Quit From Pause
  (:`Pressed`
    (if (`GameplayStatics.IsGamePaused`)
      _)))

(fn `getGameInstance`
  (returns (`Game Instance` :type "/Game/HouseOfHorror/Blueprints/BP_GameInstance Object Reference"))
  (bind _asbp_game_instance (cast `/Game/HouseOfHorror/Blueprints/BP_GameInstance` (`GameplayStatics.GetGameInstance`))
    (:`then`
      _)
    (:`CastFailed`
      _))
  (return _asbp_game_instance))

(fn `UserConstructionScript`)