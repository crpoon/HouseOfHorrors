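; BP_Scream2 is a screamer character in House of Horror that can laugh or scream, tied to a corpse slot in the CorpseManager.
; Scream plays a child's scream and publishes its position through BP_GameInstance as an active call for 1.5 seconds.
; It then clears the call, frees its corpse ID, has the manager transform it into another corpse, and destroys itself.
; SelfDestroy frees the slot silently, while SetScream switches the audio from laughing to screaming.
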(event `/Game/HouseOfHorror/Blueprints/Characters/BP_Scream.ReceiveBeginPlay`
  (`parent.ReceiveBeginPlay`))

(event `self.ReceiveEndPlay`
  (params (EndPlayReason :type "EEndPlayReason Enum" :default "Destroyed"))
  (`parent.ReceiveEndPlay` "Destroyed"))

(event `self.ReceiveActorBeginOverlap`
  (params (OtherActor :type "Actor Object Reference")))

(event `Scream`
  (bind _returnvalue (`self.K2_GetActorLocation`))
  (bind _corpsemanager (`self.CorpseManager`))
  (`AudioComponent.Stop` (`self.Audio`))
  (`GameplayStatics.PlaySoundAtLocation` "/Game/HouseOfHorror/Audio/Active/Corpses/Child_Scream-SoundBible_com-1951741114.Child_Scream-SoundBible_com-1951741114" (`self.K2_GetActorLocation`))
  (bind _asbp_game_instance (cast `/Game/HouseOfHorror/Blueprints/Utility/BP_GameInstance` (`GameplayStatics.GetGameInstance`)))
  (set `/Game/HouseOfHorror/Blueprints/Utility/BP_GameInstance.isScreamerCalling` true _asbp_game_instance)
  (set `/Game/HouseOfHorror/Blueprints/Utility/BP_GameInstance.ScreamerPosition` _returnvalue _asbp_game_instance)
  (`KismetSystemLibrary.Delay` 1.5)
  (`/Game/HouseOfHorror/Blueprints/Characters/BP_CorpseManager.SetCorpseAvailable` _corpsemanager (`self.CorpseId`))
  (set `/Game/HouseOfHorror/Blueprints/Utility/BP_GameInstance.IsScreamerCalling` false _asbp_game_instance)
  (`/Game/HouseOfHorror/Blueprints/Characters/BP_CorpseManager.TransformIntoOtherCorpse` _corpsemanager _returnvalue)
  (`self.K2_DestroyActor`))

(event `Laugh`
  (`AudioComponent.Play` (`self.Audio`) 0.0))

(event `self.ReceiveTick`
  (params (DeltaSeconds :type "Float (single-precision)"))
  (`parent.ReceiveTick` DeltaSeconds))

(fn `SelfDestroy`
  (`/Game/HouseOfHorror/Blueprints/Characters/BP_CorpseManager.SetCorpseAvailable` (`self.CorpseManager`) (`self.CorpseId`))
  (`self.K2_DestroyActor`))

(fn `SetScream`
  (params (setScreamingTo :type Boolean))
  (if (not (== setScreamingTo false))
    ;[1 1 1] If originally not screaming, set sound to screaming
    (if (== false false)
      (`AudioComponent.SetSound` (`self.Audio`) "/Game/HouseOfHorror/Audio/Active/Corpses/Child_Scream-SoundBible_com-1951741114.Child_Scream-SoundBible_com-1951741114")
      (set `self.isLaughing` false))))

(fn `UserConstructionScript`
  (`parent.UserConstructionScript`))