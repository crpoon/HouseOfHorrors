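; BP_Corpse_Creep is a zombie character whose movement speed reacts to how the player moves.
; Each tick it reads player state from BP_GameInstance, moving at triple the player's speed while they run and a fifth while they crawl.
; Otherwise, including when the player is stationary, it uses the base walk speed cached in the construction script.
; An event plays an attached sound for seeing its target.
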(event `self.ReceiveBeginPlay`
  (`parent.ReceiveBeginPlay`))

(event `self.ReceiveEndPlay`
  (params (EndPlayReason :type "EEndPlayReason Enum" :default "Destroyed"))
  (`parent.ReceiveEndPlay` "Destroyed"))

(event `self.ReceiveActorBeginOverlap`
  (params (OtherActor :type "Actor Object Reference")))

(event `self.ReceiveTick`
  (params (DeltaSeconds :type "Float (single-precision)"))
  (bind _charactermovement (`self.CharacterMovement`))
  (`parent.ReceiveTick` DeltaSeconds)
  (bind _asbp_game_instance (cast `/Game/HouseOfHorror/Blueprints/Utility/BP_GameInstance` (`GameplayStatics.GetGameInstance`)))
  (if (`/Game/HouseOfHorror/Blueprints/Utility/BP_GameInstance.isStationary` _asbp_game_instance)
    (if (`/Game/HouseOfHorror/Blueprints/Utility/BP_GameInstance.isPlayerCrawling` _asbp_game_instance) :!label _label
      (if (`/Game/HouseOfHorror/Blueprints/Utility/BP_GameInstance.isStationary` _asbp_game_instance)
        (set `CharacterMovementComponent.MaxWalkSpeed` (`self.baseWalkSpeed`) _charactermovement :!label _label_2)
        (else
          (set `CharacterMovementComponent.MaxWalkSpeed` (* (`/Game/HouseOfHorror/Blueprints/Utility/BP_GameInstance.playerCurrSpeed` _asbp_game_instance) 0.2) _charactermovement)))
      (else
        (goto _label_2)))
    (elif (`/Game/HouseOfHorror/Blueprints/Utility/BP_GameInstance.isPlayerRunning` _asbp_game_instance)
      (set `CharacterMovementComponent.MaxWalkSpeed` (* (`/Game/HouseOfHorror/Blueprints/Utility/BP_GameInstance.playerCurrSpeed` _asbp_game_instance) 3.0) (`self.CharacterMovement`))
      (else
        (goto _label)))))

(event `self.PlaySeeingTargetSound`
  ;[1 1 1] Play sound when zombie is nearby
  (`GameplayStatics.SpawnSoundAttached` (`self.SeeingTargetSound`) (`self.Audio`)))

(fn `UserConstructionScript`
  (`parent.UserConstructionScript`)
  (set `self.baseWalkSpeed` (`CharacterMovementComponent.MaxWalkSpeed` (`self.CharacterMovement`))))