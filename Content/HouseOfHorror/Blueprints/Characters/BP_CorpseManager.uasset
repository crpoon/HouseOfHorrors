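; Manager actor that spawns AI corpses near the player in House of Horror, limited to two active at once.
; A two-second timer gives a random chance to spawn one in a random neighbour of the player's room.
; Types come from a depleting ID pool, refillable through SetCorpseAvailable, and spawn with follower behavior trees.
; TransformIntoOtherCorpse spawns a replacement intended to exclude the screamer; CallCorpse's spawn branch is hard-wired off.
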(event `self.ReceiveBeginPlay`
  (`KismetSystemLibrary.K2_SetTimer` null "SpawnCorpse" 2.0 true))

(event `self.ReceiveActorBeginOverlap`
  (params (OtherActor :type "Actor Object Reference")))

(event `self.ReceiveTick`
  (params (DeltaSeconds :type "Float (single-precision)")))

(fn `CallCorpse`
  (bind _centralroom (`self.centralRoom`))
  (bind _asbp_ho_hchar (cast `/Game/HouseOfHorror/Blueprints/Character/BP_HoHChar` (`GameplayStatics.GetPlayerPawn` 0)))
  (bind _currentroom (`/Game/HouseOfHorror/Blueprints/Character/BP_HoHChar.CurrentRoom` _asbp_ho_hchar))
  (if (!= _currentroom null)
    ;[1 1 1] If current room is an intersection, select its non-intersection neighbour to be the central room
    (if (`/Game/HouseOfHorror/Blueprints/Triggers/BP_In_Room_Trigger.IsIntersection` _currentroom)
      (bind _newroom (`self.GetNonIntersectionNeighbour` _currentroom))
      (set `self.centralRoom` _newroom)
      (else
        (set `self.centralRoom` _currentroom)))
    (if (!= _centralroom null)
      (`self.GetSpawnLocation` _centralroom)
      (if false
        (`/Engine/EditorBlueprintResources/StandardMacros.IncrementInt` (`self.NumActiveCorpses`)
          (:`  `
            (bind _type (`self.GetCorpseTypeToSpawn` false))
            (`self.SpawnCorpseOfType` _type)))))))

(fn `CanSpawn`
  (params (currentRoom :type "/Game/HouseOfHorror/Blueprints/Triggers/BP_In_Room_Trigger Object Reference"))
  (returns (canSpawn :type Boolean))
  (return (and (!= currentRoom null) (< (`self.NumActiveCorpses`) 2) (> (`KismetMathLibrary.RandomFloatInRange` 0.0 1.0) 0.5))))

(fn `DecrementNumActiveCorpes`
  (`/Engine/EditorBlueprintResources/StandardMacros.DecrementInt` (`self.NumActiveCorpses`)
    (:`  `
      (return))))

(fn `GetCorpseTypeToSpawn`
  (params (excludeScreamer :type Boolean))
  (returns (type :type Integer))
  (bind _availablecorpsestocall (`self.AvailableCorpsesToCall`))
  (bind _output_get (set `self.IndexToRemove` (`KismetMathLibrary.RandomIntegerInRange` 0 (- (`KismetArrayLibrary.Array_Length` _availablecorpsestocall) 1))))
  (bind _output_get_2 (set `self.Spawning` (`KismetArrayLibrary.Array_Get` _availablecorpsestocall _output_get)))
  (`KismetArrayLibrary.Array_Remove` _availablecorpsestocall _output_get)
  (if (and excludeScreamer (== _output_get_2 3))
    (`self.GetCorpseTypeToSpawn` true)
    (`self.SetCorpseAvailable` 3))
  (return (`self.Spawning`)))

(fn `GetNonIntersectionNeighbour`
  (params (CurrentRoom :type "/Game/HouseOfHorror/Blueprints/Triggers/BP_In_Room_Trigger Object Reference"))
  (returns (NewRoom :type "/Game/HouseOfHorror/Blueprints/Triggers/BP_In_Room_Trigger Object Reference"))
  (bind _neighbours (`/Game/HouseOfHorror/Blueprints/Triggers/BP_In_Room_Trigger.Neighbours` CurrentRoom))
  ;[1 1 1] If current room is intersection, select a room that is not an intersection, or return none
  (return (`KismetArrayLibrary.Array_Get` _neighbours (`KismetMathLibrary.RandomIntegerInRange` 0 (- (`KismetArrayLibrary.Array_Length` _neighbours) 1)))))

(fn `GetSpawnLocation`
  (params (currentRoom :type "/Game/HouseOfHorror/Blueprints/Triggers/BP_In_Room_Trigger Object Reference"))
  (returns (location :type "Vector Structure"))
  (return (+ (`self.K2_GetActorLocation` currentRoom) (0.0 0.0 70.0))))

(fn `SetCorpseAvailable`
  (params (id :type Integer))
  (`KismetArrayLibrary.Array_Add` (`self.AvailableCorpsesToCall`) id))

(fn `SpawnCorpse`
  (bind _asbp_ho_hchar (cast `/Game/HouseOfHorror/Blueprints/Character/BP_HoHChar` (`GameplayStatics.GetPlayerPawn` 0)))
  (bind _currentroom (`/Game/HouseOfHorror/Blueprints/Character/BP_HoHChar.CurrentRoom` _asbp_ho_hchar))
  (if (!= _currentroom null)
    (bind _newroom (`self.GetNonIntersectionNeighbour` _currentroom))
    (bind _canspawn (`self.CanSpawn` _newroom))
    (if _canspawn
      (bind _location (`self.GetSpawnLocation` _newroom))
      (`/Engine/EditorBlueprintResources/StandardMacros.IncrementInt` (`self.NumActiveCorpses`)
        (:`  `
          (bind _type (`self.GetCorpseTypeToSpawn` false))
          (`self.SpawnCorpseOfType` _type _location))))))

(fn `SpawnCorpseOfType`
  (params (type :type Integer) (location :type "Vector Structure"))
  (returns (corpse :type "/Game/HouseOfHorror/Blueprints/Characters/BP_AICharacter Object Reference"))
  (switch `int` type
    (:`0`
      (bind _returnvalue (`AIBlueprintHelperLibrary.SpawnAIFromClass` "/Game/HouseOfHorror/Blueprints/Characters/BP_Corpse_Bob.BP_Corpse_Bob_C" "/Game/HouseOfHorror/Blueprints/AI/BehaviourTree/BT_Follower.BT_Follower" location))
      (bind _asbp_aicharacter (cast `/Game/HouseOfHorror/Blueprints/Characters/BP_AICharacter` _returnvalue)
        (:`then`
          (set `/Game/HouseOfHorror/Blueprints/Characters/BP_AICharacter.CorpseManager` self _asbp_aicharacter)
          (set `/Game/HouseOfHorror/Blueprints/Characters/BP_AICharacter.CorpseId` 0 _asbp_aicharacter)
          (return _asbp_aicharacter))
        (:`CastFailed`
          _)))
    (:`1`
      (bind _returnvalue_2 (`AIBlueprintHelperLibrary.SpawnAIFromClass` "/Game/HouseOfHorror/Blueprints/Characters/BP_Corpse_Creep.BP_Corpse_Creep_C" "/Game/HouseOfHorror/Blueprints/AI/BehaviourTree/BT_Follower.BT_Follower" location))
      (bind _asbp_aicharacter_2 (cast `/Game/HouseOfHorror/Blueprints/Characters/BP_AICharacter` _returnvalue_2)
        (:`then`
          (set `/Game/HouseOfHorror/Blueprints/Characters/BP_AICharacter.CorpseManager` self _asbp_aicharacter_2)
          (set `/Game/HouseOfHorror/Blueprints/Characters/BP_AICharacter.CorpseId` 1 _asbp_aicharacter_2)
          (return _asbp_aicharacter_2))
        (:`CastFailed`
          _)))
    (:`2`
      (bind _returnvalue_3 (`AIBlueprintHelperLibrary.SpawnAIFromClass` "/Game/HouseOfHorror/Blueprints/Characters/BP_Corpse_FormerGuard.BP_Corpse_FormerGuard_C" "/Game/HouseOfHorror/Blueprints/AI/BehaviourTree/BT_Follower.BT_Follower" location))
      (bind _asbp_aicharacter_3 (cast `/Game/HouseOfHorror/Blueprints/Characters/BP_AICharacter` _returnvalue_3)
        (:`then`
          (set `/Game/HouseOfHorror/Blueprints/Characters/BP_AICharacter.CorpseManager` self _asbp_aicharacter_3)
          (set `/Game/HouseOfHorror/Blueprints/Characters/BP_AICharacter.CorpseId` 2 _asbp_aicharacter_3)
          (return _asbp_aicharacter_3))
        (:`CastFailed`
          _)))
    (:`3`
      (bind _returnvalue_4 (`AIBlueprintHelperLibrary.SpawnAIFromClass` "/Game/HouseOfHorror/Blueprints/Characters/BP_Scream2.BP_Scream2_C" "/Game/HouseOfHorror/Blueprints/AI/BehaviourTree/BT_Follower_Screamer.BT_Follower_Screamer" location))
      (bind _asbp_aicharacter_4 (cast `/Game/HouseOfHorror/Blueprints/Characters/BP_AICharacter` _returnvalue_4)
        (:`then`
          (set `/Game/HouseOfHorror/Blueprints/Characters/BP_AICharacter.CorpseManager` self _asbp_aicharacter_4)
          (set `/Game/HouseOfHorror/Blueprints/Characters/BP_AICharacter.CorpseId` 3 _asbp_aicharacter_4)
          (return _asbp_aicharacter_4))
        (:`CastFailed`
          _))))
  (return null))

(fn `TransformIntoOtherCorpse`
  (params (location :type "Vector Structure"))
  (returns (Corpse :type "/Game/HouseOfHorror/Blueprints/Characters/BP_AICharacter Object Reference"))
  (bind _type (`self.GetCorpseTypeToSpawn` true))
  (bind _corpse (`self.SpawnCorpseOfType` _type location))
  (return _corpse))

(fn `UserConstructionScript`)