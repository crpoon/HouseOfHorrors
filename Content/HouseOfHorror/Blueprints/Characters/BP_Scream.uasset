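; BP_Scream is a House of Horror character Blueprint that plays a child's scream or giggling sound and can signal its location while screaming.
; Each tick, Scream and Laugh check their flags on a shared Audio component, restarting the matching sound when idle or silencing it when both are off.
; SetScream switches to screaming, cancelling laughter, and publishes the screaming state and actor position to BP_GameInstance whenever that state changes.
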(event `self.ReceiveBeginPlay`
  (`self.Custom Tick`))

(event `self.ReceiveActorBeginOverlap`
  (params (OtherActor :type "Actor Object Reference")))

(event `Custom Tick`)

(event `self.ReceiveTick`
  (params (DeltaSeconds :type "Float (single-precision)"))
  (`parent.ReceiveTick` 0.0)
  (`self.Scream`)
  (`self.Laugh`))

(fn `Laugh`
  (bind _audio (`self.Audio`))
  (bind _returnvalue (`AudioComponent.IsPlaying` _audio))
  (if (`self.isLaughing`)
    (if (not _returnvalue)
      ;[1 1 1] Set sound if the audio is not currently playing
      (`AudioComponent.SetSound` _audio "/Game/HouseOfHorror/Audio/Active/Corpses/Giggles-SoundBible_com-710042657.Giggles-SoundBible_com-710042657")
      (`AudioComponent.Play` _audio 0.0))
    (else
      ;[1 1 1] Fade out audio if it's currently playing
      (if (and _returnvalue (not (`self.isScreaming`)))
        (`AudioComponent.FadeOut` _audio 0.0 0.0)))))

(fn `Scream`
  (bind _audio (`self.Audio`))
  (bind _returnvalue (`AudioComponent.IsPlaying` _audio))
  (if (`self.isScreaming`)
    (if (not _returnvalue)
      ;[1 1 1] Set sound if the audio is not currently playing
      (`AudioComponent.SetSound` _audio "/Game/HouseOfHorror/Audio/Active/Corpses/Child_Scream-SoundBible_com-1951741114.Child_Scream-SoundBible_com-1951741114")
      (`AudioComponent.Play` _audio 0.0))
    (else
      ;[1 1 1] Fade out audio if it's currently playing
      (if (and _returnvalue (not (`self.isLaughing`)))
        (`AudioComponent.Stop` _audio)))))

(fn `SetScream`
  (params (setScreamingTo :type Boolean))
  (bind _isscreaming (`self.isScreaming`))
  (if (not (== setScreamingTo _isscreaming))
    ;[1 1 1] If originally not screaming, set sound to screaming
    (if (== _isscreaming false)
      (`AudioComponent.SetSound` (`self.Audio`) "/Game/HouseOfHorror/Audio/Active/Corpses/Child_Scream-SoundBible_com-1951741114.Child_Scream-SoundBible_com-1951741114")
      (set `self.isLaughing` false))
    (bind _output_get (set `self.isScreaming` setScreamingTo))
    (bind _asbp_game_instance (cast `/Game/HouseOfHorror/Blueprints/BP_GameInstance` (`GameplayStatics.GetGameInstance`)))
    (set `/Game/HouseOfHorror/Blueprints/BP_GameInstance.IsScreamerCalling` _output_get _asbp_game_instance)
    (set `/Game/HouseOfHorror/Blueprints/BP_GameInstance.ScreamerPosition` (`self.K2_GetActorLocation`) _asbp_game_instance)))

(fn `UserConstructionScript`
  (`parent.UserConstructionScript`))