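; BP_LockedDoor is a door that stays locked until the objective key has been collected.
; Its Interact event overrides the parent's and passes through to it only when the key check succeeds; otherwise it plays an attached locked-door sound.
; The HasObjectiveKeyBeenCollected macro reads a hardcoded ItemList slot in BP_GameInstance to decide.
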(event `self.ReceiveBeginPlay`)

(event `self.ReceiveActorBeginOverlap`
  (params (OtherActor :type "Actor Object Reference")))

(event `self.ReceiveTick`
  (params (DeltaSeconds :type "Float (single-precision)")))

(event `/Game/HouseOfHorror/Blueprints/Architecture/BP_Interact.Interact`
  (bind _asbp_game_instance (cast `/Game/HouseOfHorror/Blueprints/BP_GameInstance` (`GameplayStatics.GetGameInstance`)))
  (if (`KismetArrayLibrary.Array_Get` (`/Game/HouseOfHorror/Blueprints/BP_GameInstance.itemList` _asbp_game_instance) 1)
    (`parent.Interact`)
    (else
      (`GameplayStatics.SpawnSoundAttached` "/Game/HouseOfHorror/Audio/Active/Door/SC_LockedDoor.SC_LockedDoor" (`self.DefaultSceneRoot`)))))

(fn `UserConstructionScript`
  (`parent.UserConstructionScript`))