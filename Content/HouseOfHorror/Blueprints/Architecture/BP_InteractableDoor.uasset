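; Interactable door Blueprint that swings open or shut by 90 degrees of yaw when its Interact event fires.
; IsOpen selects the OpenDoor or CloseDoor graph, each of which drives SetActorRotation through a timeline, relative to the yaw captured at the start.
; When the timeline finishes, IsOpen flips and a DoOnce resets, so interactions during a swing are ignored.
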(event `/Game/HouseOfHorror/Blueprints/Architecture/BP_Interact.Interact`
  (bind (_returnvalue_roll _returnvalue_pitch _returnvalue_yaw) (`KismetMathLibrary.BreakRotator` (`self.K2_GetActorRotation`)))
  (bind (_returnvalue_roll_2 _returnvalue_pitch_2 _returnvalue_yaw_2) (`KismetMathLibrary.BreakRotator` (`self.K2_GetActorRotation`)))
  (`/Engine/EditorBlueprintResources/StandardMacros.DoOnce` false :!label _label
    (:`Completed`
      (if (`self.isOpen`)
        (set `self.zRotation` _returnvalue_yaw)
        (bind (_direction _close) (`Timeline|Close` :!via `PlayFromStart`)
          (:`Update`
            (`self.SetActorRotation` (`KismetMathLibrary.MakeRotator` 0.0 0.0 (+ (* _close -90.0) (`self.zRotation`)))))
          (:`Finished`
            (`self.ToggleisOpen` :!label _label_2)
            (`|ExecutionSequence`
              (:`then_0`
                (goto _label :!via `Reset`)))))
        (else
          (set `self.zRotation` _returnvalue_yaw_2)
          (bind (_direction_2 _open) (`Timeline|Open` :!via `PlayFromStart`)
            (:`Update`
              (`self.SetActorRotation` (`KismetMathLibrary.MakeRotator` 0.0 0.0 (+ (* _open 90.0) (`self.zRotation`)))))
            (:`Finished`
              (goto _label_2))))))))

(fn `ToggleisOpen`
  (set `self.isOpen` (not (`self.isOpen`)))
  (return))

(fn `UserConstructionScript`
  (`parent.UserConstructionScript`))