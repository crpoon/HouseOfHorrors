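; Creeping corpse enemy that adjusts its walk speed to how the player is moving.
; Each Tick it reads player state from BP_GameInstance, moving at a multiple of the player's speed while they run and a fraction of it while they crawl.
; Otherwise, including when the player is stationary, it uses the base walk speed cached in the Construction Script.
; Two helper macros count running or crawling only while the player is not stationary.
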(event `self.ReceiveBeginPlay`)

(event `self.ReceiveActorBeginOverlap`
  (params (OtherActor :type "Actor Object Reference")))

(event `self.ReceiveTick`
  (params (DeltaSeconds :type "Float (single-precision)"))
  (bind _charactermovement (`self.CharacterMovement`))
  (bind _asbp_game_instance (cast `/Game/HouseOfHorror/Blueprints/BP_GameInstance` (`GameplayStatics.GetGameInstance`)))
  (if (`/Game/HouseOfHorror/Blueprints/BP_GameInstance.isStationary` _asbp_game_instance)
    (if (`/Game/HouseOfHorror/Blueprints/BP_GameInstance.isPlayerCrawling` _asbp_game_instance) :!label _label
      (if (`/Game/HouseOfHorror/Blueprints/BP_GameInstance.isStationary` _asbp_game_instance)
        (set `CharacterMovementComponent.MaxWalkSpeed` (`self.baseWalkSpeed`) _charactermovement :!label _label_2)
        (else
          (set `CharacterMovementComponent.MaxWalkSpeed` (* (`/Game/HouseOfHorror/Blueprints/BP_GameInstance.playerCurrSpeed` _asbp_game_instance) 0.2) _charactermovement)))
      (else
        (goto _label_2)))
    (elif (`/Game/HouseOfHorror/Blueprints/BP_GameInstance.isPlayerRunning` _asbp_game_instance)
      (set `CharacterMovementComponent.MaxWalkSpeed` (* (`/Game/HouseOfHorror/Blueprints/BP_GameInstance.playerCurrSpeed` _asbp_game_instance) 3.0) (`self.CharacterMovement`))
      (else
        (goto _label)))))

(fn `UserConstructionScript`
  (`parent.UserConstructionScript`)
  (set `self.baseWalkSpeed` (`CharacterMovementComponent.MaxWalkSpeed` (`self.CharacterMovement`))))