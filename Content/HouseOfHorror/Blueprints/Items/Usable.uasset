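; Base pickup-and-use item for House of Horror that the player can collect into the HUD inventory.
; The construction script applies the custom mesh and fills the item's inventory struct with its image and texts.
; A sphere trigger toggles a pickup prompt widget and in-range flag for the player's bound pickup event.
; Pickup adds the struct to the inventory, disables collision and refreshes the HUD, while UseAction only prints a placeholder message.
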(event `self.ReceiveBeginPlay`
  (bind _iteminfo (`self.ItemInfo`))
  (bind (_item _itemimage _pickuptest) (break `/Game/HouseOfHorror/Blueprints/InventorySystem/InventoryStruct` _iteminfo))
  (bind _returnvalue (`|CreateWidget` "/Game/HouseOfHorror/Blueprints/InventorySystem/PickupText.PickupText_C"))
  (set `self.PickupTextWidget` _returnvalue)
  (set `/Game/HouseOfHorror/Blueprints/InventorySystem/PickupText.PickupActor` _item _returnvalue)
  (set `/Game/HouseOfHorror/Blueprints/InventorySystem/PickupText.PickupText` _pickuptest _returnvalue) ; Set text
  (setmembers `/Game/HouseOfHorror/Blueprints/InventorySystem/InventoryStruct` :`StructRef` _iteminfo :`Item` self)
  (bind _asbp_ho_hchar (cast `/Game/HouseOfHorror/Blueprints/Character/BP_HoHChar` (`GameplayStatics.GetPlayerCharacter` 0)))
  (set `self.Player` _asbp_ho_hchar)
  (add `/Game/HouseOfHorror/Blueprints/Character/BP_HoHChar.PickUpItem` _asbp_ho_hchar (delegate `PickUpItem_Event_0`)))

(event `self.ReceiveActorBeginOverlap`
  (params (OtherActor :type "Actor Object Reference")))

(event `self.ReceiveTick`
  (params (DeltaSeconds :type "Float (single-precision)")))

(event `PickUpItem_Event_0`
  (bind _gamehudwidget (`/Game/HouseOfHorror/Blueprints/Character/BP_HoHChar.GameHUDWidget` (`self.Player`)))
  ;[1 1 1] Pickup and Add To Inventory
  (if (and (`self.GetActorEnableCollision`) (`self.IsInRange`))
    (`KismetArrayLibrary.Array_Add` (`/Game/HouseOfHorror/Blueprints/Utility/GameHUD.Inventory` _gamehudwidget) (`self.ItemInfo`))
    (`Widget.RemoveFromParent` (`self.PickupTextWidget`))
    (`self.SetActorHiddenInGame` false)
    (`self.SetActorEnableCollision` false)
    (`/Game/HouseOfHorror/Blueprints/Utility/GameHUD.RefreshInventory` _gamehudwidget)))

(event `self.Sphere.OnComponentBeginOverlap`
  (params (OtherActor :type "Actor Object Reference") (OtherComp :type "PrimitiveComponent Object Reference") (OtherBodyIndex :type Integer) (bFromSweep :type Boolean) (SweepResult :type "HitResult Structure (by ref)"))
  ;[1 1 1] Triggers
  (cast `/Game/HouseOfHorror/Blueprints/Character/BP_HoHChar` OtherActor)
  (`UserWidget.AddToViewport` (`self.PickupTextWidget`) 0)
  (set `self.IsInRange` true))

(event `self.Sphere.OnComponentEndOverlap`
  (params (OtherActor :type "Actor Object Reference") (OtherComp :type "PrimitiveComponent Object Reference") (OtherBodyIndex :type Integer))
  ;[1 1 1] Triggers
  (cast `/Game/HouseOfHorror/Blueprints/Character/BP_HoHChar` OtherActor)
  (`Widget.RemoveFromParent` (`self.PickupTextWidget`))
  (set `self.IsInRange` false))

(event `/Game/HouseOfHorror/Blueprints/InventorySystem/ActionInterface.UseAction`
  (`KismetSystemLibrary.PrintString` "Item used!"))

(fn `UserConstructionScript`
  (setmembers `/Game/HouseOfHorror/Blueprints/InventorySystem/InventoryStruct` :`StructRef` (`self.ItemInfo`) :`Item` self :`ItemImage` (`self.InventoryImage`) :`PickupTest` (`self.PickupText`) :`ActionTest` (`self.ActionText`))
  (`StaticMeshComponent.SetStaticMesh` (`self.StaticMesh`) (`self.CustomMesh`)))