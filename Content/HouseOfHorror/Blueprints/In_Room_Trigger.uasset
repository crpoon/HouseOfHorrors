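; Room trigger volume for the House of Horror game that tracks which room the player and AI corpses occupy.
; On box overlap it sets itself as CurrentRoom on the player or AI character and prints its RoomName, plus its neighbour count for the player.
; On exit it clears the player's CurrentRoom unconditionally, while AI characters keep their last room.
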(event `self.ReceiveBeginPlay`)

(event `self.ReceiveActorBeginOverlap`
  (params (OtherActor :type "Actor Object Reference")))

(event `self.ReceiveTick`
  (params (DeltaSeconds :type "Float (single-precision)")))

(event `self.Box.OnComponentBeginOverlap`
  (params (OtherActor :type "Actor Object Reference") (OtherComp :type "PrimitiveComponent Object Reference") (OtherBodyIndex :type Integer) (bFromSweep :type Boolean) (SweepResult :type "HitResult Structure (by ref)"))
  (bind _asbp_ho_hchar (cast `/Game/HouseOfHorror/Blueprints/Character/BP_HoHChar` OtherActor)
    (:`then`
      (bind _output_get (set `/Game/HouseOfHorror/Blueprints/Character/BP_HoHChar.CurrentRoom` self _asbp_ho_hchar))
      (`KismetSystemLibrary.PrintString` (`KismetStringLibrary.Concat_StrStr` "Player at: " (`/Game/HouseOfHorror/Blueprints/In_Room_Trigger.RoomName` _output_get) ", numbr of neighbouring rooms: " (`KismetStringLibrary.Conv_IntToString` (`KismetArrayLibrary.Array_Length` (`/Game/HouseOfHorror/Blueprints/In_Room_Trigger.Neighbours` _output_get)))) true true (struct :`G` 0.66 :`B` 1.0 :`A` 1.0) 5.0))
    (:`CastFailed`
      (bind _asbp_aicharacter (cast `/Game/HouseOfHorror/Blueprints/Characters/BP_AICharacter` OtherActor))
      (bind _output_get_2 (set `/Game/HouseOfHorror/Blueprints/Characters/BP_AICharacter.CurrentRoom` self _asbp_aicharacter))
      (`KismetSystemLibrary.PrintString` (`KismetStringLibrary.Concat_StrStr` "Corpse at: " (`/Game/HouseOfHorror/Blueprints/In_Room_Trigger.RoomName` _output_get_2)) true true (struct :`G` 0.66 :`B` 1.0 :`A` 1.0) 5.0))))

(event `self.Box.OnComponentEndOverlap`
  (params (OtherActor :type "Actor Object Reference") (OtherComp :type "PrimitiveComponent Object Reference") (OtherBodyIndex :type Integer))
  (bind _asbp_ho_hchar (cast `/Game/HouseOfHorror/Blueprints/Character/BP_HoHChar` OtherActor))
  (set `/Game/HouseOfHorror/Blueprints/Character/BP_HoHChar.CurrentRoom` null _asbp_ho_hchar))

(fn `UserConstructionScript`)